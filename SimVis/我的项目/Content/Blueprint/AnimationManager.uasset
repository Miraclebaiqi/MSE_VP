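; AnimationManager turns text commands into robot actions for a simulated ABB-style industrial arm cell (IRB6700_270, IRB2600_185).
; A command switch sends robots to preset poses, grabs or drops parts, or forwards assembly to Statemanager and welding to TimeNodeManager.
; Grabbed actors follow the arm's Link6 each Tick at a stored offset.
; Drops teleport parts to a DropPoint that steps along X, then send the robot home.
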(event Custom|select%20animation
  (params (command :type String) (robot :type Robot%20Object%20Reference) (rescource :type Actor%20Object%20Reference) (condtion :type Actor%20Object%20Reference))
  ;[1 1 1] 根据命令-动画判定
  (switch string command
    (:Default
      (Development|PrintString "命令格式错误，请检查拼写" true true "(R=1.000000,G=0.000000,B=0.000000,A=1.000000)" 6e+01))
    (:move1
      (CallFunction|MovetoRes1 robot))
    (:move2
      (CallFunction|MovetoRes2 robot))
    (:movep
      (CallFunction|MovetoP robot))
    (:move3
      (CallFunction|MovetoPout robot))
    (:move0
      (CallFunction|MovetoO robot))
    (:grab
      (CallFunction|Grab robot rescource))
    (:drop2
      (CallFunction|Drop robot rescource :!label _label))
    (:drop3
      (goto _label))
    (:anzhuang
      (bind _outactors (Actor|GetAllActorsOfClass "/Game/Blueprint/Statemanager.Statemanager_C"))
      (Default|Anzhuang (Utilities|Array|Get(acopy) _outactors) rescource condtion))
    (:hanjie
      (bind _outactors_2 (Actor|GetAllActorsOfClass "/Game/Blueprint/TimeNodeManager.TimeNodeManager_C"))
      (Default|CurrentNodeFinished (Utilities|Array|Get(acopy) _outactors_2)))))

(event Custom|Grab
  (params (robot :type Robot%20Object%20Reference) (Actor :type Actor%20Object%20Reference))
  (bind _asirb6700_270 (Utilities|Casting|CastToIRB6700_270 robot))
  (bind _output_get (Variables|Default|SetGrabRobot _asirb6700_270))
  (Variables|Default|SetGrabActor Actor)
  (Variables|Default|SetOffset (- (Transformation|GetActorLocation Actor) (Transformation|GetWorldLocation (Variables|/Game/Blueprint/IRB6700_270.IRB6700_270_C|Getlink6 _output_get))))
  (Variables|Default|SetIsGrab true)
  (CallFunction|MovetoO _output_get))

(event Custom|Drop
  (params (robot :type Actor%20Object%20Reference) (Drop%20actor :type Actor%20Object%20Reference))
  (bind _asirb6700_270 (Utilities|Casting|CastToIRB6700_270 robot))
  (Variables|Default|SetIsGrab false)
  (Transformation|SetActorLocation Drop%20actor (Variables|Default|GetDropPoint) false false)
  (Variables|Default|SetDropPoint (+ (Variables|Default|GetDropPoint) "189.000000,0.000000,0.000000"))
  (CallFunction|MovetoO _asirb6700_270))

(event Custom|Move%20To%20Res1
  (params (robot :type Robot%20Object%20Reference))
  (bind _asirb6700_270 (Utilities|Casting|CastToIRB6700_270 robot))
  (Default|Moveto _asirb6700_270 (Variables|/Game/Blueprint/IRB6700_270.IRB6700_270_C|Getpose_pin_res1 _asirb6700_270)))

(event Custom|Move%20To%20P
  (params (robot :type Robot%20Object%20Reference))
  (bind _asirb6700_270 (Utilities|Casting|CastToIRB6700_270 robot)
    (:then
      (Default|Moveto _asirb6700_270 (Variables|/Game/Blueprint/IRB6700_270.IRB6700_270_C|Getpose_p _asirb6700_270)))
    (:CastFailed
      (bind _asirb2600_185 (Utilities|Casting|CastToIRB2600_185 robot))
      (Default|Moveto _asirb2600_185 (Variables|/Game/Blueprint/IRB2600_185.IRB2600_185_C|Getpose_p _asirb2600_185)))))

(event Custom|Move%20To%20Pout
  (params (robot :type Robot%20Object%20Reference))
  (bind _asirb6700_270 (Utilities|Casting|CastToIRB6700_270 robot))
  (Default|Moveto _asirb6700_270 (Variables|/Game/Blueprint/IRB6700_270.IRB6700_270_C|Getpose_pout _asirb6700_270)))

(event Custom|Move%20To%20Res2
  (params (robot :type Robot%20Object%20Reference))
  (bind _asirb6700_270 (Utilities|Casting|CastToIRB6700_270 robot))
  (Default|Moveto _asirb6700_270 (Variables|/Game/Blueprint/IRB6700_270.IRB6700_270_C|Getpose_res2 _asirb6700_270)))

(event Custom|Move%20to%20O
  (params (robot :type Robot%20Object%20Reference))
  (bind _asirb6700_270 (Utilities|Casting|CastToIRB6700_270 robot)
    (:then
      (Default|Moveto _asirb6700_270 (Variables|/Game/Blueprint/IRB6700_270.IRB6700_270_C|Getpose_o _asirb6700_270)))
    (:CastFailed
      (bind _asirb2600_185 (Utilities|Casting|CastToIRB2600_185 robot))
      (Default|Moveto _asirb2600_185 (Variables|/Game/Blueprint/IRB2600_185.IRB2600_185_C|Getpose_o _asirb2600_185)))))

(event EventTick
  (params (DeltaSeconds :type Float%20%28single-precision%29))
  (bind _grabactor (Variables|Default|GetGrabActor))
  (if (Variables|Default|GetIsGrab)
    (if (Utilities|IsValid _grabactor)
      (Transformation|SetActorLocation _grabactor (+ (Transformation|GetWorldLocation (Variables|/Game/Blueprint/IRB6700_270.IRB6700_270_C|Getlink6 (Variables|Default|GetGrabRobot))) (Variables|Default|GetOffset)) false false))))

(fn ConstructionScript)
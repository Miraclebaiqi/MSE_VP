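; IRB6700_270 is a six-axis robot arm actor that animates from its current joint pose to a target pose.
; MoveTo caches each link's single-axis relative rotation into PoseCurrent, then a timeline linearly interpolates the six joints toward TargetPose.
; When the timeline finishes, it prints a completion message and calls CurrentNodeFinished on the first TimeNodeManager found in the level.
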(event Custom|MoveTo
  (params (target%20pose :type Array%20of%20Floats%20%28double-precision%29))
  (CallFunction|GetCurrentPose)
  (bind _alpha (Timeline|MoveTo_Timeline PlayFromStart)
    (:Update
      (CallFunction|MovetoNewPose target%20pose _alpha))
    (:Finished
      (Development|PrintString "动作完成" true true "(R=0.000000,G=1.000000,B=0.042499,A=1.000000)" 5.0)
      (bind _outactors (Actor|GetAllActorsOfClass "/Game/Blueprint/TimeNodeManager.TimeNodeManager_C"))
      (Default|CurrentNodeFinished (Utilities|Array|Get(acopy) _outactors)))))

(event EventBeginPlay)

(event Collision|EventActorBeginOverlap
  (params (OtherActor :type Actor%20Object%20Reference)))

(event EventTick
  (params (DeltaSeconds :type Float%20%28single-precision%29)))

(fn ConstructionScript)

(fn GetCurrentPose
  (Utilities|Array|SetArrayElem (Variables|Default|Getpose_current) 1 (.yaw (Variables|/Script/Engine.SceneComponent|GetRelativeRotation (Variables|Default|Getlink1))))
  (Utilities|Array|SetArrayElem (Variables|Default|Getpose_current) 2 (.pitch (Variables|/Script/Engine.SceneComponent|GetRelativeRotation (Variables|Default|Getlink2))))
  (Utilities|Array|SetArrayElem (Variables|Default|Getpose_current) 3 (.pitch (Variables|/Script/Engine.SceneComponent|GetRelativeRotation (Variables|Default|Getlink3))))
  (Utilities|Array|SetArrayElem (Variables|Default|Getpose_current) 4 (.roll (Variables|/Script/Engine.SceneComponent|GetRelativeRotation (Variables|Default|Getlink4))))
  (Utilities|Array|SetArrayElem (Variables|Default|Getpose_current) 5 (.pitch (Variables|/Script/Engine.SceneComponent|GetRelativeRotation (Variables|Default|Getlink5))))
  (Utilities|Array|SetArrayElem (Variables|Default|Getpose_current) 6 (.roll (Variables|/Script/Engine.SceneComponent|GetRelativeRotation (Variables|Default|Getlink6)))))

(fn MovetoNewPose
  (params (NewPose :type Array%20of%20Floats%20%28double-precision%29) (Alpha :type Float%20%28double-precision%29))
  (bind _pose_current (Variables|Default|Getpose_current))
  (Transformation|SetRelativeRotation (Variables|Default|Getlink1) (Math|Rotator|MakeRotator 0.0 0.0 (Math|Float|Lerp (Utilities|Array|Get(acopy) _pose_current 1) (Utilities|Array|Get(acopy) NewPose 1) Alpha)) false false)
  (Transformation|SetRelativeRotation (Variables|Default|Getlink2) (Math|Rotator|MakeRotator 0.0 (Math|Float|Lerp (Utilities|Array|Get(acopy) _pose_current 2) (Utilities|Array|Get(acopy) NewPose 2) Alpha) 0.0) false false)
  (Transformation|SetRelativeRotation (Variables|Default|Getlink3) (Math|Rotator|MakeRotator 0.0 (Math|Float|Lerp (Utilities|Array|Get(acopy) _pose_current 3) (Utilities|Array|Get(acopy) NewPose 3) Alpha) 0.0) false false)
  (Transformation|SetRelativeRotation (Variables|Default|Getlink4) (Math|Rotator|MakeRotator (Math|Float|Lerp (Utilities|Array|Get(acopy) _pose_current 4) (Utilities|Array|Get(acopy) NewPose 4) Alpha) 0.0 0.0) false false)
  (Transformation|SetRelativeRotation (Variables|Default|Getlink5) (Math|Rotator|MakeRotator 0.0 (Math|Float|Lerp (Utilities|Array|Get(acopy) _pose_current 5) (Utilities|Array|Get(acopy) NewPose 5) Alpha) 0.0) false false)
  (Transformation|SetRelativeRotation (Variables|Default|Getlink6) (Math|Rotator|MakeRotator (Math|Float|Lerp (Utilities|Array|Get(acopy) _pose_current 6) (Utilities|Array|Get(acopy) NewPose 6) Alpha) 0.0 0.0) false false))
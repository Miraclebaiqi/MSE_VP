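; TimeNode is a robot command step that drives the first IRB6700_270 arm in its Robots array.
; ExecuteRobotCommands handles Move, Grab and Drop, with Grab attaching Res to Link6 and Drop detaching it, both keeping world transforms.
; Move lerps each of the six links on its single joint axis from Opose to Pose by a supplied Alpha.
; A DoOnce in Initial captures Opose from the arm's current joint rotations.
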(event Custom|initial
  (bind _robots (Variables|Default|Getrobots))
  (Utilities|FlowControl|DoOnce false
    (:Completed
      (if (> (Utilities|Array|Length _robots) 0)
        (bind _asirb6700_270 (Utilities|Casting|CastToIRB6700_270 (Utilities|Array|Get(acopy) _robots)))
        (Variables|Default|SetOpose (Utilities|Struct|MakeRobot_Pose (.yaw (.rotation (Transformation|GetRelativeTransform (Variables|/Game/Blueprint/IRB6700_270.IRB6700_270_C|Getlink1 _asirb6700_270)))) (.pitch (.rotation (Transformation|GetRelativeTransform (Variables|/Game/Blueprint/IRB6700_270.IRB6700_270_C|Getlink2 _asirb6700_270)))) (.pitch (.rotation (Transformation|GetRelativeTransform (Variables|/Game/Blueprint/IRB6700_270.IRB6700_270_C|Getlink3 _asirb6700_270)))) (.roll (.rotation (Transformation|GetRelativeTransform (Variables|/Game/Blueprint/IRB6700_270.IRB6700_270_C|Getlink4 _asirb6700_270)))) (.pitch (.rotation (Transformation|GetRelativeTransform (Variables|/Game/Blueprint/IRB6700_270.IRB6700_270_C|Getlink5 _asirb6700_270)))) (.roll (.rotation (Transformation|GetRelativeTransform (Variables|/Game/Blueprint/IRB6700_270.IRB6700_270_C|Getlink6 _asirb6700_270))))))))))

(event EventBeginPlay)

(event Collision|EventActorBeginOverlap
  (params (OtherActor :type Actor%20Object%20Reference)))

(event EventTick
  (params (DeltaSeconds :type Float%20%28single-precision%29)))

(fn ConstructionScript)

(fn ExecuteRobotCommands
  (params (Alpha :type Float%20%28double-precision%29) (command :type String))
  (bind _robots (Variables|Default|Getrobots))
  (bind _pose (Variables|Default|Getpose))
  (bind _robots_2 (Variables|Default|Getrobots))
  (bind _opose (Variables|Default|GetOpose))
  (bind _robots_3 (Variables|Default|Getrobots))
  (switch string command
    (:move
      (if (> (Utilities|Array|Length _robots_2) 0)
        (bind _asirb6700_270 (Utilities|Casting|CastToIRB6700_270 (Utilities|Array|Get(acopy) _robots_2)))
        (Utilities|FlowControl|Sequence
          (:then_0
            (CallFunction|Initial))
          (:then_1
            (Transformation|SetRelativeRotation (Variables|/Game/Blueprint/IRB6700_270.IRB6700_270_C|Getlink1 _asirb6700_270) (Math|Rotator|MakeRotator 0.0 0.0 (Math|Float|Lerp (.link1 _opose) (.link1 _pose) Alpha)) false false)
            (Transformation|SetRelativeRotation (Variables|/Game/Blueprint/IRB6700_270.IRB6700_270_C|Getlink2 _asirb6700_270) (Math|Rotator|MakeRotator 0.0 (Math|Float|Lerp (.link2 _opose) (.link2 _pose) Alpha) 0.0) false false)
            (Transformation|SetRelativeRotation (Variables|/Game/Blueprint/IRB6700_270.IRB6700_270_C|Getlink3 _asirb6700_270) (Math|Rotator|MakeRotator 0.0 (Math|Float|Lerp (.link3 _opose) (.link3 _pose) Alpha) 0.0) false false)
            (Transformation|SetRelativeRotation (Variables|/Game/Blueprint/IRB6700_270.IRB6700_270_C|Getlink4 _asirb6700_270) (Math|Rotator|MakeRotator (Math|Float|Lerp (.link4 _opose) (.link4 _pose) Alpha) 0.0 0.0) false false)
            (Transformation|SetRelativeRotation (Variables|/Game/Blueprint/IRB6700_270.IRB6700_270_C|Getlink5 _asirb6700_270) (Math|Rotator|MakeRotator 0.0 (Math|Float|Lerp (.link5 _opose) (.link5 _pose) Alpha) 0.0) false false)
            (Transformation|SetRelativeRotation (Variables|/Game/Blueprint/IRB6700_270.IRB6700_270_C|Getlink6 _asirb6700_270) (Math|Rotator|MakeRotator (Math|Float|Lerp (.link6 _opose) (.link6 _pose) Alpha) 0.0 0.0) false false)))))
    (:grab
      (if (Utilities|IsValid (Variables|Default|GetRes))
        (if (> (Utilities|Array|Length _robots_3) 0)
          (bind _asirb6700_270_2 (Utilities|Casting|CastToIRB6700_270 (Utilities|Array|Get(acopy) _robots_3)))
          (Transformation|AttachComponentToComponent (Variables|Default|GetRes) (Variables|/Game/Blueprint/IRB6700_270.IRB6700_270_C|Getlink6 _asirb6700_270_2) "None" "KeepWorld" "KeepWorld" "KeepWorld" true))))
    (:drop
      (if (Utilities|IsValid (Variables|Default|GetRes))
        (if (> (Utilities|Array|Length _robots) 0)
          (Utilities|Casting|CastToIRB6700_270 (Utilities|Array|Get(acopy) _robots))
          (Transformation|DetachFromActor (Variables|Default|GetRes) "KeepWorld" "KeepWorld" "KeepWorld"))))))
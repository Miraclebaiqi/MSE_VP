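; Level2Base is a base Blueprint for a robotic assembly scene, with events that move workpieces Res1 and Res2 alongside robot arms and assemble them.
; Offset events record each part's position relative to Link5 of Robot1 or Robot21, and Tick uses Attach flags to make parts follow, simulating attachment without parenting.
; Installation destroys Res2 and reveals Res1's ChejiaF component, while positioning events snap Res1 to fixed stations along Y.
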(event Custom|计算偏移2
  (Variables|Default|Setoffset2 (- (Transformation|GetActorLocation (Variables|Default|Getres2)) (Transformation|GetWorldLocation (Variables|/Game/Blueprint/IRB6700_270.IRB6700_270_C|Getlink5 (Variables|Default|Getrobot_1))))))

(event Custom|模拟附加2
  (Transformation|SetActorLocation (Variables|Default|Getres2) (+ (Transformation|GetWorldLocation (Variables|/Game/Blueprint/IRB6700_270.IRB6700_270_C|Getlink5 (Variables|Default|Getrobot_1))) (Variables|Default|Getoffset2)) false false))

(event Custom|模拟附加1
  (Transformation|SetActorLocation (Variables|Default|Getres1) (+ (Transformation|GetWorldLocation (Variables|/Game/Blueprint/IRB6700_270.IRB6700_270_C|Getlink5 (Variables|Default|Getrobot_1))) (Variables|Default|Getoffset1)) false false))

(event Custom|组合件定位操作
  (Transformation|SetActorLocation (Variables|Default|Getres1) "10000.000000,10250.000000,0.000000" false false))

(event Custom|定位2_1
  (Transformation|SetActorLocation (Variables|Default|Getres1) "10000.000000,10430.000000,0.000000" false false))

(event Custom|计算偏移1_2
  (Variables|Default|Setoffset1 (- (Transformation|GetActorLocation (Variables|Default|Getres1)) (Transformation|GetWorldLocation (Variables|/Game/Blueprint/IRB6700_270.IRB6700_270_C|Getlink5 (Variables|Default|Getrobot_2_1))))))

(event Custom|模拟附加1_2
  (Transformation|SetActorLocation (Variables|Default|Getres1) (+ (Transformation|GetWorldLocation (Variables|/Game/Blueprint/IRB6700_270.IRB6700_270_C|Getlink5 (Variables|Default|Getrobot_2_1))) (Variables|Default|Getoffset1)) false false))

(event Custom|安装操作
  (Actor|DestroyActor (Variables|Default|Getres2))
  (Rendering|SetVisibility (Variables|/Game/Blueprint/chejia.chejia_C|Getchejia%28F%29 (Variables|Default|Getres1)) true false))

(event Custom|定位2_2
  (Transformation|SetActorLocation (Variables|Default|Getres1) "10000.000000,10600.000000,0.000000" false false))

(event Custom|计算偏移1
  (Variables|Default|Setoffset1 (- (Transformation|GetActorLocation (Variables|Default|Getres1)) (Transformation|GetWorldLocation (Variables|/Game/Blueprint/IRB6700_270.IRB6700_270_C|Getlink5 (Variables|Default|Getrobot_1))))))

(event EventTick
  (params (DeltaSeconds :type Float%20%28single-precision%29))
  (Utilities|FlowControl|Sequence
    (:then_0
      (if (Variables|Default|GetAttach1)
        (CallFunction|模拟附加1)))
    (:then_1
      (if (Variables|Default|GetAttach2)
        (CallFunction|模拟附加2)))
    (:then_2
      (if (Variables|Default|GetAttach3)
        (CallFunction|模拟附加12)))))

(fn ConstructionScript)
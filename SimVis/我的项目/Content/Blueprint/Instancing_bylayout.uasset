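; Blueprint that builds a scene from the Layout_specification_data DataTable, spawning one actor per recognized row at its stored position and rotation.
; The Instancing event switches on category: Resource spawns a Zongcheng, stores the model as ResName and shows the matching panel or door component.
; Point spawns a marker, while Robot picks an IRB 6700 or IRB 2600 class by model and assigns its RobotID.
; Unknown categories and completion are reported with PrintString.
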(event Custom|Instancing
  (bind _outrownames (DataTable|GetDataTableRowNames "/Game/Data/Layout_specification_data.Layout_specification_data"))
  (for _array_element _outrownames
    (bind _returnvalue (Utilities|GetDataTableRow "/Game/Data/Layout_specification_data.Layout_specification_data" _array_element)
      (:then
        (switch string (.category _returnvalue)
          (:Default
            (Development|PrintString (Utilities|String|Append "未找到对应的实例化类型：" (.category _returnvalue)) true true "(R=1.000000,G=0.000000,B=0.000000,A=1.000000)" 6e+01))
          (:resource
            (bind _returnvalue_2 (Game|SpawnActorfromClass "/Game/Blueprint/zongcheng.zongcheng_C" (Math|Transform|MakeTransform (Math|Vector|MakeVector (.pos_x _returnvalue) (.pos_y _returnvalue) (.pos_z _returnvalue)) (Math|Rotator|MakeRotator (.rot_x _returnvalue) (.rot_y _returnvalue) (.rot_z _returnvalue)) "1.000000,1.000000,1.000000") "Undefined" "MultiplyWithRoot" 0 0))
            (Variables|/Game/Blueprint/zongcheng.zongcheng_C|SetResName _returnvalue_2 (.model _returnvalue))
            (switch string (.model _returnvalue)
              (:qiandiban
                (Rendering|SetVisibility (Variables|/Game/Blueprint/zongcheng.zongcheng_C|Getqiandiban _returnvalue_2) true false))
              (:houdiban
                (Rendering|SetVisibility (Variables|/Game/Blueprint/zongcheng.zongcheng_C|Gethoudiban _returnvalue_2) true false))
              (:qianweiban
                (Rendering|SetVisibility (Variables|/Game/Blueprint/zongcheng.zongcheng_C|Getqianweiban _returnvalue_2) true false))
              (:zuocewei
                (Rendering|SetVisibility (Variables|/Game/Blueprint/zongcheng.zongcheng_C|Getleftdoor _returnvalue_2) true false))
              (:youcewei
                (Rendering|SetVisibility (Variables|/Game/Blueprint/zongcheng.zongcheng_C|Getrightdoor _returnvalue_2) true false))
              (:dingbu
                (Rendering|SetVisibility (Variables|/Game/Blueprint/zongcheng.zongcheng_C|Getding _returnvalue_2) true false))))
          (:point
            (Game|SpawnActorfromClass "/Game/Blueprint/Point.Point_C" (Math|Transform|MakeTransform (Math|Vector|MakeVector (.pos_x _returnvalue) (.pos_y _returnvalue) (.pos_z _returnvalue)) (Math|Rotator|MakeRotator (.rot_x _returnvalue) (.rot_y _returnvalue) (.rot_z _returnvalue)) "1.000000,1.000000,1.000000") "Undefined" "MultiplyWithRoot" 0 0))
          (:robot
            (switch string (.model _returnvalue)
              (:IRB_6700
                (bind _returnvalue_3 (Game|SpawnActorfromClass "/Game/Blueprint/IRB6700_270.IRB6700_270_C" (Math|Transform|MakeTransform (Math|Vector|MakeVector (.pos_x _returnvalue) (.pos_y _returnvalue) (.pos_z _returnvalue)) (Math|Rotator|MakeRotator (.rot_x _returnvalue) (.rot_y _returnvalue) (.rot_z _returnvalue)) "1.000000,1.000000,1.000000") "Undefined" "MultiplyWithRoot" 0 0))
                (Variables|/Game/Blueprint/Robot.Robot_C|SetrobotID _returnvalue_3 (.id _returnvalue)))
              (:IRB_2600
                (bind _returnvalue_4 (Game|SpawnActorfromClass "/Game/Blueprint/IRB2600_185.IRB2600_185_C" (Math|Transform|MakeTransform (Math|Vector|MakeVector (.pos_x _returnvalue) (.pos_y _returnvalue) (.pos_z _returnvalue)) (Math|Rotator|MakeRotator (.rot_x _returnvalue) (.rot_y _returnvalue) (.rot_z _returnvalue)) "1.000000,1.000000,1.000000") "Undefined" "MultiplyWithRoot" 0 0))
                (Variables|/Game/Blueprint/Robot.Robot_C|SetrobotID _returnvalue_4 (.id _returnvalue)))))))))
  (Development|PrintString "实例化完成" true true "(R=0.000000,G=1.000000,B=1.000000,A=1.000000)" 5.0))

(fn ConstructionScript)
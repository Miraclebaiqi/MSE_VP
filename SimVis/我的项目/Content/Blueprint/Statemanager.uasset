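; Statemanager handles part installation (anzhuang) in what appears to be a vehicle body assembly sequence built from zongcheng actors.
; The install event casts both the major and sub actor to zongcheng, then switches on the sub's ResName to reveal the matching hidden component on the major, such as floor panels, doors or roof.
; It then destroys the sub actor and tells the first TimeNodeManager found that the current node is finished.
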(event Custom|anzhuang
  (params (major :type Actor%20Object%20Reference) (sub :type Actor%20Object%20Reference))
  (bind _aszongcheng (Utilities|Casting|CastTozongcheng major))
  (bind _aszongcheng_2 (Utilities|Casting|CastTozongcheng sub))
  (switch string (Variables|/Game/Blueprint/zongcheng.zongcheng_C|GetResName _aszongcheng_2)
    (:qiandiban
      (Rendering|SetVisibility (Variables|/Game/Blueprint/zongcheng.zongcheng_C|Getqiandiban _aszongcheng) true false))
    (:houdiban
      (Rendering|SetVisibility (Variables|/Game/Blueprint/zongcheng.zongcheng_C|Gethoudiban _aszongcheng) true false))
    (:qianweiban
      (Rendering|SetVisibility (Variables|/Game/Blueprint/zongcheng.zongcheng_C|Getqianweiban _aszongcheng) true false))
    (:zuocewei
      (Rendering|SetVisibility (Variables|/Game/Blueprint/zongcheng.zongcheng_C|Getleftdoor _aszongcheng) true false))
    (:youcewei
      (Rendering|SetVisibility (Variables|/Game/Blueprint/zongcheng.zongcheng_C|Getrightdoor _aszongcheng) true false))
    (:dingbu
      (Rendering|SetVisibility (Variables|/Game/Blueprint/zongcheng.zongcheng_C|Getding _aszongcheng) true false)))
  (Actor|DestroyActor _aszongcheng_2)
  (bind _outactors (Actor|GetAllActorsOfClass "/Game/Blueprint/TimeNodeManager.TimeNodeManager_C"))
  (Default|CurrentNodeFinished (Utilities|Array|Get(acopy) _outactors)))

(fn ConstructionScript)